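; Game instance for a two-player platformer that carries scores and music across rounds.
; On map load it starts the music once, then a tick later restores each BP_PlatformingCharacter's score and updates its HUD.
; SavePlayerScore stores the score, flags a win at three points and starts a short timer.
; The timer removes the second player, then reloads StarterMap or, on a win, opens WinLevel and stops the music.
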(event Custom|OpenLevel
  (Class|GameplayStatics|RemovePlayer (Game|GetPlayerController 1) false)
  (if (Variables|Default|GetAnyoneWon?)
    (Game|OpenLevel(byName) "WinLevel")
    (Audio|Components|Audio|Stop (Variables|Default|GetGameMusicRef))
    (else
      (Game|OpenLevel(byName) " StarterMap"))))

(event EventGameMapLoaded
  (if (Variables|Default|GetShould%20Play%20Music)
    (bind _returnvalue (Audio|SpawnSound2D "/Game/Sounds/bombel__Edit_1_Export_1_Cue.bombel__Edit_1_Export_1_Cue" 1.0 1.0 0.0 0 true))
    (Variables|Default|SetGameMusicRef _returnvalue)
    (Variables|Default|SetShould%20Play%20Music false))
  (Utilities|FlowControl|DelayUntilNextTick)
  (for _index (range 0 1)
    (bind _asbp_platforming_character (Utilities|Casting|CastToBP_PlatformingCharacter (Game|Player|GetPlayerPawn _index)))
    (bind _output_get (Variables|/Game/Blueprints/BP_PlatformingCharacter.BP_PlatformingCharacter_C|SetScore _asbp_platforming_character (Utilities|Select :Index _index :Option%200 (Variables|Default|GetPlayer1Score) :Option%201 (Variables|Default|GetPlayer2Score))))
    (Default|IncreaseScore (Variables|/Game/Blueprints/BP_PlatformingCharacter.BP_PlatformingCharacter_C|GetHUD%20ref _asbp_platforming_character) _output_get _index)))

(event EventSavePlayerScore
  (params (Player%20Score :type Integer) (Player%20Index :type Integer))
  (Variables|Default|SetAnyoneWon? (== Player%20Score 3))
  (switch int Player%20Index
    (:0
      (Variables|Default|SetPlayer1Score Player%20Score))
    (:1
      (Variables|Default|SetPlayer2Score Player%20Score)))
  (Utilities|Time|SetTimerbyEvent (delegate Custom|OpenLevel) 2.0))