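; GM_Platformer is a game mode, judging by its name, that sets up local multiplayer on BeginPlay.
; It gathers all PlayerStarts, creates an additional local player with its own controller, then teleports each player's pawn to the start at the matching array index.
; Inside that per-player loop it also looks up the user of every connected input device, but the result is unused.
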(event EventBeginPlay
  (bind _outactors (Actor|GetAllActorsOfClass "/Script/Engine.PlayerStart"))
  (Variables|Default|SetPlayerStarts _outactors)
  (Class|GameplayStatics|CreatePlayer -1)
  (bind _returnvalue (Class|GameModeBase|GetNumPlayers))
  (for _index (range 0 (- _returnvalue 1))
    (Transformation|SetActorTransform (Game|Player|GetPlayerPawn _index) (Transformation|GetActorTransform (Utilities|Array|Get(acopy) (Variables|Default|GetPlayerStarts) _index)) false true)
    (bind _outinputdevices (Class|InputDeviceLibrary|GetAllConnectedInputDevices))
    (for _array_element _outinputdevices
      (Class|InputDeviceLibrary|GetUserforInputDevice _array_element))))

(fn ConstructionScript)