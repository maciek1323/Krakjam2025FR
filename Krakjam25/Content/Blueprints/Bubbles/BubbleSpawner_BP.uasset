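; BubbleSpawner_BP is a spawner actor that periodically creates Bubble_BP actors of random size.
; BeginPlay starts a one-shot timer that fires SpawnNewBubble after IntervalTime.
; While Active, each spawn picks a random integer radius and a random X within SpawningBounds, keeps the spawner's Y and Z, then re-arms the timer.
; If Active is false when the timer fires, the cycle stops.
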(event Custom|Spawn%20new%20bubble
  (bind _returnvalue (Transformation|GetActorLocation))
  (bind _spawningbounds (Variables|Default|GetSpawningBounds))
  (if (Variables|Default|GetActive?)
    (Variables|Default|SetBubbleRadius (Math|Random|RandomIntegerinRange 20 80))
    (Game|SpawnActorfromClass "/Game/Blueprints/Bubbles/Bubble_BP.Bubble_BP_C" (Math|Transform|MakeTransform (Math|Vector|MakeVector (Math|Random|RandomFloatinRange (.X (Math|Vector|BreakVector (Utilities|Array|Get(acopy) _spawningbounds))) (.X (Math|Vector|BreakVector (Utilities|Array|Get(acopy) _spawningbounds 1)))) (.y _returnvalue) (.z _returnvalue)) "0, 0, 0" "1.000000,1.000000,1.000000") "Undefined" "MultiplyWithRoot" 0 (Variables|Default|GetBubbleRadius) 0)
    (Utilities|Time|SetTimerbyEvent (delegate Custom|Spawn%20new%20bubble) (Variables|Default|GetIntervalTime))))

(event EventBeginPlay
  (Utilities|Time|SetTimerbyEvent (delegate Custom|Spawn%20new%20bubble) (Variables|Default|GetIntervalTime)))

(fn ConstructionScript)