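; Bubble actor that drifts upward and bounces the player into the air on contact.
; Tick moves it up a fixed step per frame, without sweep or delta-time scaling.
; Sphere overlap sends an upward launch through BPI_PlayerCharacter, with LaunchForce scaled by the Felek curve sampled at BubbleRadius, then destroys the bubble.
; The construction script scales only the Plane from BubbleRadius.
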(event OnComponentBeginOverlap(Sphere)
  (params (OverlappedComponent :type Primitive%20Component%20Object%20Reference) (OtherActor :type Actor%20Object%20Reference) (OtherComp :type Primitive%20Component%20Object%20Reference) (OtherBodyIndex :type Integer) (bFromSweep :type Boolean) (SweepResult :type Hit%20Result%20Structure%20%28by%20ref%29))
  (if (Utilities|DoesObjectImplementInterface OtherActor "/Game/Interfaces/BPI_PlayerCharacter.BPI_PlayerCharacter_C")
    (Class|BPIPlayerCharacter|LaunchPlayer(Message) OtherActor (Math|Vector|MakeVector 0.0 0.0 (Math|Conversions|ToFloat(Integer) (* (Math|Curves|GetFloatValue (Variables|Default|GetFelek) (Math|Conversions|ToFloat(Integer) (Variables|Default|GetBubbleRadius))) (Variables|Default|GetLaunchForce)))))
    (Actor|DestroyActor)))

(event EventBeginPlay)

(event Collision|EventActorBeginOverlap
  (params (OtherActor :type Actor%20Object%20Reference)))

(event EventTick
  (params (DeltaSeconds :type Float%20%28single-precision%29))
  (Transformation|AddActorWorldOffset "0.000000,0.000000,1.000000"))

(fn ConstructionScript
  (bind _bubbleradius (Variables|Default|GetBubbleRadius))
  (Transformation|SetRelativeScale3D (Variables|Default|GetPlane) (* (Math|Vector|MakeVector (Math|Conversions|ToFloat(Integer) _bubbleradius) (Math|Conversions|ToFloat(Integer) _bubbleradius) (Math|Conversions|ToFloat(Integer) _bubbleradius)) 0.01)))