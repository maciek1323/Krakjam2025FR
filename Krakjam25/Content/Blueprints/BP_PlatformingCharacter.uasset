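; BP_PlatformingCharacter is a player-controlled platformer character that moves along the world X axis and jumps.
; On BeginPlay it registers the Platformer_MappingContext with the Enhanced Input subsystem of its player controller.
; IA_Move feeds movement input scaled by MovementSpeed, while IA_Jump starts and stops the built-in Character jump.
; The OnJumped and OnLanded events maintain a Jumping flag.
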(event Input|EnhancedActionEvents|EnhancedInputActionIA_Move
  (params (ActionValue :type Float%20%28double-precision%29) (ElapsedSeconds :type Float%20%28double-precision%29) (TriggeredSeconds :type Float%20%28double-precision%29) (InputAction :type Input%20Action%20Object%20Reference :default "/Game/Input/InputActions/IA_Move.IA_Move"))
  (Pawn|Input|AddMovementInput (Math|Vector|MakeVector (* (Variables|Default|GetMovement%20Speed) ActionValue) 0.0 0.0) 1.0 false))

(event Input|EnhancedActionEvents|EnhancedInputActionIA_Jump
  (params (ActionValue :type Boolean) (ElapsedSeconds :type Float%20%28double-precision%29) (TriggeredSeconds :type Float%20%28double-precision%29) (InputAction :type Input%20Action%20Object%20Reference :default "/Game/Input/InputActions/IA_Jump.IA_Jump"))
  (:Triggered
    (Character|Jump))
  (:Completed
    (Character|StopJumping)))

(event EventBeginPlay
  (bind _asplayer_controller (Utilities|Casting|CastToPlayerController (Pawn|GetController)))
  (Input|AddMappingContext (PlayerController|LocalPlayerSubsystems|GetEnhancedInputLocalPlayerSubsystem _asplayer_controller) "/Game/Input/Platformer_MappingContext.Platformer_MappingContext" 0 "(bIgnoreAllPressedKeysUntilRelease=True,bForceImmediately=False,bNotifyUserSettings=False)"))

(event EventOnJumped
  (Variables|Default|SetJumping true))

(event EventOnLanded
  (params (Hit :type Hit%20Result%20Structure%20%28by%20ref%29))
  (Variables|Default|SetJumping false))

(fn ConstructionScript)