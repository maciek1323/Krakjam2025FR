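; BP_WinScreenCharacters is a flipbook character for the win screen that shows a winning or losing player animation.
; On BeginPlay it reads Player 1's score from the Jezyk_GI game instance to decide whether orange or green won, with three or more meaning orange.
; Its Place variable then selects the winner's win flipbook or the other color's lose flipbook.
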(event EventBeginPlay
  (bind _asjezyk_gi (Utilities|Casting|CastToJezyk_GI (Game|GetGameInstance)))
  (if (>= (Variables|/Game/Blueprints/Jezyk_GI.Jezyk_GI_C|GetPlayer1Score _asjezyk_gi) 3)
    (Sprite|SetFlipbook (Variables|Default|GetPaperFlipbook) (Utilities|Select :Index (- (Variables|Default|GetPlace) 1) :Option%200 "/Game/Sprites/Textures/FB_ORANGE_WIN.FB_ORANGE_WIN" :Option%201 "/Game/Sprites/Textures/FB_GREEB_LOSE.FB_GREEB_LOSE"))
    (else
      (Sprite|SetFlipbook (Variables|Default|GetPaperFlipbook) (Utilities|Select :Index (- (Variables|Default|GetPlace) 1) :Option%200 "/Game/Sprites/Textures/FB_GREEN_WIN.FB_GREEN_WIN" :Option%201 "/Game/Sprites/Textures/FB_ORANGE_LOSE.FB_ORANGE_LOSE")))))

(fn ConstructionScript)